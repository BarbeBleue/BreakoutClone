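; Game mode for a ball game that manages score, lives, game state and the level reset loop.
; On BeginPlay it creates the GUI widget, then resets by reloading the streamed Level1, restoring lives and score, and firing the ResetPlayerPosition and StartGame dispatchers.
; Score updates clamp at zero and push to the GUI.
; A lost ball costs points and a life; with none left, game over triggers a delayed reset.
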(event Custom|Lost%20Ball
  ;[1 1 1] Ball Lost
  (CallFunction|UpdateScore -1e+03)
  (if (<= (Variables|Default|GetpLife) 0.0)
    (CallFunction|GameOver)
    (else
      (Variables|Default|SetpLife (- (Variables|Default|GetpLife) 1.0))
      (Variables|/Game/Blueprints/gui.gui_C|SetpLife (Variables|Default|GetGUI) (Variables|Default|GetpLife)))))

(event Custom|Game%20Over
  ;[1 1 1] Game over
  (Variables|Default|SetEGameStates "NewEnumerator1")
  (Utilities|FlowControl|Delay 5.0)
  (CallFunction|ResetGame))

(event Custom|Load%20Level
  (bind _returnvalue (Utilities|Name|MakeLiteralName "Level1"))
  ;[1 1 1] Load Level
  (Game|UnloadStreamLevel(byName) _returnvalue)
  (Game|LoadStreamLevel(byName) _returnvalue true))

(event Custom|Reset%20Game
  (bind _maxlifes (Variables|Default|GetMaxLifes))
  (bind _gui (Variables|Default|GetGUI))
  (Development|PrintString "Hello")
  (CallFunction|LoadLevel)
  (Variables|Default|SetpLife _maxlifes)
  (Variables|/Game/Blueprints/gui.gui_C|SetpLife _gui _maxlifes)
  (Variables|/Game/Blueprints/gui.gui_C|SetScore _gui 0.0)
  (Variables|Default|SetCurrent%20Score 0.0)
  (Default|CallResetPlayerPosition)
  (Variables|Default|SetEGameStates "NewEnumerator0")
  (Default|CallStartGame))

(event Custom|Update%20Score
  (params (Points :type Float%20%28single-precision%29))
  ;[1 1 1] Update Score
  (if (< (+ Points (Variables|Default|GetCurrent%20Score)) 0.0)
    (Variables|Default|SetCurrent%20Score 0.0)
    (else
      (Variables|Default|SetCurrent%20Score (+ Points (Variables|Default|GetCurrent%20Score)))))
  (Variables|/Game/Blueprints/gui.gui_C|SetScore (Variables|Default|GetGUI) (Variables|Default|GetCurrent%20Score)))

(event EventBeginPlay
  ;[1 1 1] Add GUI
  (bind _returnvalue (UserInterface|CreateWidget "/Game/Blueprints/gui.gui_C"))
  (bind _output_get (Variables|Default|SetGUI _returnvalue))
  (UserInterface|Viewport|AddtoViewport _output_get 0)
  (CallFunction|ResetGame))

(fn ConstructionScript)