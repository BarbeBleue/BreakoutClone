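; Physics ball actor that travels at a fixed speed along diagonals in the XY plane.
; BeginPlay launches it with a diagonal velocity-change impulse.
; Every Tick, it clamps velocity magnitude to Speed and rebuilds the direction from yaw alone, flattening vertical motion.
; It snaps that yaw by rotating 45 degrees, rounding to 90-degree steps and rotating back, so any deflection resolves to one of four diagonals.
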(event Custom|Launch
  ;[1 1 1] Launch ball
  (Physics|AddImpulse (Variables|Default|GetBall) "500.000000,-500.000000, 0" "None" true))

(event Custom|Clamp%20Velocity
  (bind _returnvalue (Transformation|GetVelocity))
  (bind _returnvalue_2 (Math|Rotator|MakeRotator 0.0 0.0 45.0))
  (bind _speed (Variables|Default|GetSpeed))
  (bind _returnvalue_3 (Math|Vector|ClampVectorSize _returnvalue _speed _speed))
  ;[1 1 1] clamp ball velocity
  (Physics|SetPhysicsLinearVelocity (Variables|Default|GetBall) (* (Math|Vector|UnrotateVector (Math|Rotator|GetRotationXVector (Math|Rotator|MakeRotator 0.0 0.0 (|((round((A/B)))*B) (.yaw (Math|Rotator|MakeRotfromX (Math|Vector|RotateVector _returnvalue_3 _returnvalue_2))) 9e+01))) _returnvalue_2) (Math|Vector|VectorLength _returnvalue_3)) false "None"))

(event EventBeginPlay
  (CallFunction|Launch))

(event EventTick
  (params (DeltaSeconds :type Float%20%28single-precision%29))
  (CallFunction|ClampVelocity))

(fn ConstructionScript)