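; Player-controlled paddle that moves horizontally and launches a ball.
; On BeginPlay it caches OurGameMode and its start location, then binds to the game mode's reset-position and start-game events to reposition itself or spawn a ball at its Arrow.
; Horizontal input pushes the paddle with physics impulses; movement and spawning require a specific game state.
; Fire launches a valid, inactive ball along the Arrow's forward vector.
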(event Custom|ResetPlayerPosition
  (bind _playerstartlocation (Variables|Default|GetPlayerStartLocation))
  ;[1 1 1] Reset Player Position
  (Transformation|SetActorLocation _playerstartlocation false false)
  (Transformation|SetWorldLocation (Variables|Default|GetPaddle) _playerstartlocation false false))

(event Custom|Spawn%20New%20Ball
  ;[1 1 1] Spawn New Ball
  (if (Utilities|Enum|Equal(Enum) (Variables|/Game/Blueprints/OurGameMode.OurGameMode_C|GetEGameStates (Variables|Default|GetGameMode)) "NewEnumerator0")
    (bind _returnvalue (Game|SpawnActorfromClass "/Game/Blueprints/Ball.Ball_C" (Transformation|GetWorldTransform (Variables|Default|GetArrow)) "AlwaysSpawn" 0 0))
    (Variables|Default|SetBall _returnvalue)))

(event EventBeginPlay
  ;[1 1 1] Get Game Mode
  (bind _asour_game_mode (Utilities|Casting|CastToOurGameMode (Game|GetGameMode)))
  (Variables|Default|SetGameMode _asour_game_mode)
  ;[1 1 1] Save Player Start Location
  (Variables|Default|SetPlayerStartLocation (Transformation|GetActorLocation))
  ;[1 1 1] Bind Events
  (EventDispatchers|BindEventtoResetPlayerPosition (Variables|Default|GetGameMode) (delegate Custom|ResetPlayerPosition))
  (EventDispatchers|BindEventtoStartGame (Variables|Default|GetGameMode) (delegate Custom|Spawn%20New%20Ball)))

(event Input|ActionEvents|InputActionFire
  (params (Key :type Key%20Structure :default "AnyKey"))
  (bind _ball (Variables|Default|GetBall))
  ;[1 1 1] Launch Ball
  (:Pressed
    (if (and (Utilities|IsValid _ball) (not (Variables|/Game/Blueprints/Ball.Ball_C|GetActive _ball)))
      (Default|Launch _ball (Math|Rotator|GetRotationXVector (Transformation|GetWorldRotation (Variables|Default|GetArrow)))))))

(event Input|AxisEvents|InputAxisMoveHorizontal
  (params (AxisValue :type Float%20%28single-precision%29))
  ;[1 1 1] movement
  (if (Utilities|Enum|Equal(Enum) (Variables|/Game/Blueprints/OurGameMode.OurGameMode_C|GetEGameStates (Variables|Default|GetGameMode)) "NewEnumerator0")
    (Physics|AddImpulse (Variables|Default|GetPaddle) (Math|Vector|MakeVector (* AxisValue (Variables|Default|Getspeed)) 0.0 0.0) "None" false)))

(fn ConstructionScript)